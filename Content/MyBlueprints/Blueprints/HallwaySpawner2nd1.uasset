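; Procedural hallway spawner for the second level that places the next piece at its OpenCollider shortly after BeginPlay, aligned to its own facing.
; It spawns HallwayEnd2nd at GI_Nightmare's hallway limit; otherwise it increments the count, calls GM_Definitive's Check2ndLevelTurns and picks randomly from Hallways2ndLoopArray.
; Corner component tags on the spawned piece increment the game mode's Right or Left turn counters.
; Spawns fail rather than overlap when colliding.
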(event EventBeginPlay
  (bind _returnvalue (Transformation|GetActorRotation))
  (bind _opencollider (Variables|Default|GetOpenCollider))
  (bind _returnvalue_2 (Math|Rotator|GetRotationXVector _returnvalue))
  (bind _returnvalue_3 (Transformation|GetWorldLocation _opencollider))
  (bind _returnvalue_4 (Math|Vector|MakeVector (.x _returnvalue_3) (.y _returnvalue_3) 0.0))
  (bind _returnvalue_5 (+ "0, 0, 0" _returnvalue_2))
  (bind _returnvalue_6 (Math|Conversions|RotationFromXVector _returnvalue_5))
  (Utilities|FlowControl|Delay 0.1)
  (bind _asgi_nightmare (Utilities|Casting|CastToGI_Nightmare (Game|GetGameInstance)))
  (bind _asgm_definitive (Utilities|Casting|CastToGM_Definitive (Game|GetGameMode)))
  (if (== (Variables|/Game/MyBlueprints/Blueprints/GameModes/GI_Nightmare.GI_Nightmare_C|GetActualHallways _asgi_nightmare) (Variables|/Game/MyBlueprints/Blueprints/GameModes/GI_Nightmare.GI_Nightmare_C|GetMaxHallways _asgi_nightmare))
    (Game|SpawnActorfromClass "/Game/MyBlueprints/Blueprints/Actors/HallwayEnd2nd.HallwayEnd2nd_C" (Math|Transform|MakeTransform _returnvalue_4 _returnvalue_6 "1,1,1") "DontSpawnIfColliding" 0 0)
    (else
      (Math|Integer|IncrementInt (Variables|/Game/MyBlueprints/Blueprints/GameModes/GI_Nightmare.GI_Nightmare_C|GetActualHallways _asgi_nightmare)
        (:%20%20
          (Default|Check2ndLevelTurns _asgm_definitive)
          (bind _returnvalue_7 (Game|SpawnActorfromClass (Utilities|Array|Get(acopy) (Variables|/Game/MyBlueprints/Blueprints/GameModes/GM_Definitive.GM_Definitive_C|GetHallways2ndLoopArray _asgm_definitive) (Math|Random|RandomIntegerinRange 0 (- (Utilities|Array|Length (Variables|/Game/MyBlueprints/Blueprints/GameModes/GM_Definitive.GM_Definitive_C|GetHallways2ndLoopArray _asgm_definitive)) 1))) (Math|Transform|MakeTransform _returnvalue_4 _returnvalue_6 "1,1,1") "DontSpawnIfColliding" 0 0))
          (Utilities|IsValid _returnvalue_7
            (:Is%20Valid
              (bind _asgm_definitive_2 (Utilities|Casting|CastToGM_Definitive (Game|GetGameMode)))
              (if (Components|ComponentHasTag (Variables|/Script/Engine.Actor|GetRootComponent _returnvalue_7) "EsquinaDerecha")
                (Math|Integer|IncrementInt (Variables|/Game/MyBlueprints/Blueprints/GameModes/GM_Definitive.GM_Definitive_C|GetRight _asgm_definitive_2))
                (elif (Components|ComponentHasTag (Variables|/Script/Engine.Actor|GetRootComponent _returnvalue_7) "EsquinaIzquierda")
                  (Math|Integer|IncrementInt (Variables|/Game/MyBlueprints/Blueprints/GameModes/GM_Definitive.GM_Definitive_C|GetLeft _asgm_definitive_2)))))
            (:Is%20Not%20Valid
              (Development|PrintString (Utilities|GetDisplayName _returnvalue_7)))))))))

(fn ConstructionScript)