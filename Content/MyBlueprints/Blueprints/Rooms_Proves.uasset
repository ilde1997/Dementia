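; Rooms_Proves is a room Blueprint holding prototype logic for chaining randomly chosen rooms, though that logic is not connected to any event.
; The unwired logic compares the room count in GI_Nightmare to its maximum and increments it while they differ.
; It then spawns a random class from GM_Proves' RoomsArray at a fixed offset, skipping the spawn if collision cannot be resolved.
; BeginPlay and the construction script are empty.
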(event EventBeginPlay)

(fn ConstructionScript)