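; Game mode for the first loop, holding the hallway class list and left/right turn counters.
; CheckTurns compares the counters and, when one side leads, swaps the last four HallwaysArray entries for four copies of that side's HallwayTurns entry.
; It then zeroes both counters, while a tie changes nothing.
; BeginPlay only clears EmptyRooms; a debug print of the hallway list is left unwired.
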(event EventBeginPlay
  (Utilities|Array|Clear (Variables|Default|GetEmptyRooms)))

(event EventTick
  (params (DeltaSeconds :type Float%20%28single-precision%29)))

(fn ConstructionScript)

(fn CheckTurns
  (bind _hallwaysarray (Variables|Default|GetHallwaysArray))
  (bind _returnvalue (Utilities|Array|Length _hallwaysarray))
  (bind _returnvalue_2 (Utilities|Array|Length _hallwaysarray))
  (if (>= (+ (Variables|Default|GetLeft) (* (Variables|Default|GetRight) -1)) 1)
    (while (< (Variables|Default|GetContador) 4)
      (Utilities|Array|RemoveIndex _hallwaysarray (- _returnvalue_2 1))
      (Math|Integer|IncrementInt (Variables|Default|GetContador)))
    (Variables|Default|SetContador 0)
    (while (< (Variables|Default|GetContador) 4)
      (Utilities|Array|Insert _hallwaysarray (Utilities|Array|Get(acopy) (Variables|Default|GetHallwayTurns)) (- _returnvalue_2 0))
      (Math|Integer|IncrementInt (Variables|Default|GetContador)))
    (Variables|Default|SetRight 0 :!label _label)
    (Variables|Default|SetLeft 0)
    (Variables|Default|SetContador 0)
    (elif (>= (+ (* (Variables|Default|GetLeft) -1) (Variables|Default|GetRight)) 1)
      (while (< (Variables|Default|GetContador) 4)
        (Utilities|Array|RemoveIndex _hallwaysarray (- _returnvalue 1))
        (Math|Integer|IncrementInt (Variables|Default|GetContador)))
      (Variables|Default|SetContador 0)
      (while (< (Variables|Default|GetContador) 4)
        (Utilities|Array|Insert _hallwaysarray (Utilities|Array|Get(acopy) (Variables|Default|GetHallwayTurns) 1) (- _returnvalue 0))
        (Math|Integer|IncrementInt (Variables|Default|GetContador)))
      (goto _label))))