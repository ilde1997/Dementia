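; Game mode for a looping-hallway game that biases each loop level's hallway pool to counter or follow turn imbalance.
; BeginPlay clears empty rooms and GI_Nightmare's hallway/room counters, plus key, frame and turn state if the key had spawned.
; CheckLevelsTurns picks a per-level check, which swaps the array's last four hallways for one turn type when Left and Right differ.
; The fourth level's check exists but is not wired in.
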(event EventBeginPlay
  (Utilities|Array|Clear (Variables|Default|GetEmptyRooms))
  (bind _asgi_nightmare (Utilities|Casting|CastToGI_Nightmare (Game|GetGameInstance)))
  (Variables|/Game/MyBlueprints/Blueprints/GameModes/GI_Nightmare.GI_Nightmare_C|SetActualHallways _asgi_nightmare 0)
  (Variables|/Game/MyBlueprints/Blueprints/GameModes/GI_Nightmare.GI_Nightmare_C|SetActualRooms _asgi_nightmare 0)
  (Variables|/Game/MyBlueprints/Blueprints/GameModes/GI_Nightmare.GI_Nightmare_C|SetTutorialActualHallways _asgi_nightmare 0)
  (if (Variables|/Game/MyBlueprints/Blueprints/GameModes/GI_Nightmare.GI_Nightmare_C|GetKeyHasSpawned _asgi_nightmare)
    (Variables|/Game/MyBlueprints/Blueprints/GameModes/GI_Nightmare.GI_Nightmare_C|SetKeyHasSpawned _asgi_nightmare false)
    (Variables|/Game/MyBlueprints/Blueprints/GameModes/GI_Nightmare.GI_Nightmare_C|SetFrameHasFallen _asgi_nightmare false)
    (Variables|Default|SetRight 0)
    (Variables|Default|SetLeft 0)
    (Variables|Default|SetContador 0)))

(event EventTick
  (params (DeltaSeconds :type Float%20%28single-precision%29)))

(fn ConstructionScript)

(fn CheckLevelsTurns
  (bind _returnvalue (Game|GetCurrentLevelName true))
  (if (Utilities|Enum|Equal(Enum) _returnvalue (Variables|Levels|GetLevel_1Loop))
    (CallFunction|Check1stLevelTurns)
    (elif (Utilities|Enum|Equal(Enum) _returnvalue (Variables|Levels|GetLevel_2Loop))
      (CallFunction|Check2ndLevelTurns)
      (elif (Utilities|Enum|Equal(Enum) _returnvalue (Variables|Levels|GetLevel_3Loop))
        (CallFunction|Check3rdLevelTurns)
        (elif (Utilities|Enum|Equal(Enum) _returnvalue (Variables|Levels|GetLevel_4Loop))
          _)))))

(fn Check1stLevelTurns
  (bind _hallways1stlooparray (Variables|1stLoop|GetHallways1stLoopArray))
  (bind _returnvalue (Utilities|Array|Length _hallways1stlooparray))
  (bind _returnvalue_2 (Utilities|Array|Length _hallways1stlooparray))
  (if (>= (+ (Variables|Default|GetLeft) (* (Variables|Default|GetRight) -1)) 1)
    (while (< (Variables|Default|GetContador) 4)
      (Utilities|Array|RemoveIndex _hallways1stlooparray (- _returnvalue_2 1))
      (Math|Integer|IncrementInt (Variables|Default|GetContador)))
    (Variables|Default|SetContador 0)
    (while (< (Variables|Default|GetContador) 4)
      (Utilities|Array|Insert _hallways1stlooparray (Utilities|Array|Get(acopy) (Variables|1stLoop|GetHallway1stLoopTurns)) (- _returnvalue_2 0))
      (Math|Integer|IncrementInt (Variables|Default|GetContador)))
    (Variables|Default|SetRight 0 :!label _label)
    (Variables|Default|SetLeft 0)
    (Variables|Default|SetContador 0)
    (elif (>= (+ (* (Variables|Default|GetLeft) -1) (Variables|Default|GetRight)) 1)
      (while (< (Variables|Default|GetContador) 4)
        (Utilities|Array|RemoveIndex _hallways1stlooparray (- _returnvalue 1))
        (Math|Integer|IncrementInt (Variables|Default|GetContador)))
      (Variables|Default|SetContador 0)
      (while (< (Variables|Default|GetContador) 4)
        (Utilities|Array|Insert _hallways1stlooparray (Utilities|Array|Get(acopy) (Variables|1stLoop|GetHallway1stLoopTurns) 1) (- _returnvalue 0))
        (Math|Integer|IncrementInt (Variables|Default|GetContador)))
      (goto _label))))

(fn Check2ndLevelTurns
  (bind _hallways2ndlooparray (Variables|2ndLoop|GetHallways2ndLoopArray))
  (bind _returnvalue (Utilities|Array|Length _hallways2ndlooparray))
  (bind _returnvalue_2 (Utilities|Array|Length _hallways2ndlooparray))
  (if (>= (+ (Variables|Default|GetLeft) (* (Variables|Default|GetRight) -1)) 1)
    (while (< (Variables|Default|GetContador) 4)
      (Utilities|Array|RemoveIndex _hallways2ndlooparray (- _returnvalue_2 1))
      (Math|Integer|IncrementInt (Variables|Default|GetContador)))
    (Variables|Default|SetContador 0)
    (while (< (Variables|Default|GetContador) 4)
      (Utilities|Array|Insert _hallways2ndlooparray (Utilities|Array|Get(acopy) (Variables|2ndLoop|GetHallway2ndLoopTurns)) (- _returnvalue_2 0))
      (Math|Integer|IncrementInt (Variables|Default|GetContador)))
    (Variables|Default|SetRight 0 :!label _label)
    (Variables|Default|SetLeft 0)
    (Variables|Default|SetContador 0)
    (elif (>= (+ (* (Variables|Default|GetLeft) -1) (Variables|Default|GetRight)) 1)
      (while (< (Variables|Default|GetContador) 4)
        (Utilities|Array|RemoveIndex _hallways2ndlooparray (- _returnvalue 1))
        (Math|Integer|IncrementInt (Variables|Default|GetContador)))
      (Variables|Default|SetContador 0)
      (while (< (Variables|Default|GetContador) 4)
        (Utilities|Array|Insert _hallways2ndlooparray (Utilities|Array|Get(acopy) (Variables|2ndLoop|GetHallway2ndLoopTurns) 1) (- _returnvalue 0))
        (Math|Integer|IncrementInt (Variables|Default|GetContador)))
      (goto _label))))

(fn Check3rdLevelTurns
  (bind _hallways3rdlooparray (Variables|3rdLoop|GetHallways3rdLoopArray))
  (bind _returnvalue (Utilities|Array|Length _hallways3rdlooparray))
  (bind _returnvalue_2 (Utilities|Array|Length _hallways3rdlooparray))
  (if (>= (+ (Variables|Default|GetLeft) (* (Variables|Default|GetRight) -1)) 1)
    (while (< (Variables|Default|GetContador) 4)
      (Utilities|Array|RemoveIndex _hallways3rdlooparray (- _returnvalue_2 1))
      (Math|Integer|IncrementInt (Variables|Default|GetContador)))
    (Variables|Default|SetContador 0)
    (while (< (Variables|Default|GetContador) 4)
      (Utilities|Array|Insert _hallways3rdlooparray (Utilities|Array|Get(acopy) (Variables|3rdLoop|GetHallway3rdLoopTurns)) (- _returnvalue_2 0))
      (Math|Integer|IncrementInt (Variables|Default|GetContador)))
    (Variables|Default|SetRight 0 :!label _label)
    (Variables|Default|SetLeft 0)
    (Variables|Default|SetContador 0)
    (elif (>= (+ (* (Variables|Default|GetLeft) -1) (Variables|Default|GetRight)) 1)
      (while (< (Variables|Default|GetContador) 4)
        (Utilities|Array|RemoveIndex _hallways3rdlooparray (- _returnvalue 1))
        (Math|Integer|IncrementInt (Variables|Default|GetContador)))
      (Variables|Default|SetContador 0)
      (while (< (Variables|Default|GetContador) 4)
        (Utilities|Array|Insert _hallways3rdlooparray (Utilities|Array|Get(acopy) (Variables|3rdLoop|GetHallway3rdLoopTurns) 1) (- _returnvalue 0))
        (Math|Integer|IncrementInt (Variables|Default|GetContador)))
      (goto _label))))

(fn Check4thLevelTurns
  (bind _hallways4thlooparray (Variables|4thLoop|GetHallways4thLoopArray))
  (bind _returnvalue (Utilities|Array|Length _hallways4thlooparray))
  (bind _returnvalue_2 (Utilities|Array|Length _hallways4thlooparray))
  (if (>= (+ (Variables|Default|GetLeft) (* (Variables|Default|GetRight) -1)) 1)
    (while (< (Variables|Default|GetContador) 4)
      (Utilities|Array|RemoveIndex _hallways4thlooparray (- _returnvalue_2 1))
      (Math|Integer|IncrementInt (Variables|Default|GetContador)))
    (Variables|Default|SetContador 0)
    (while (< (Variables|Default|GetContador) 4)
      (Utilities|Array|Insert _hallways4thlooparray (Utilities|Array|Get(acopy) (Variables|4thLoop|GetHallway4thLoopTurns)) (- _returnvalue_2 0))
      (Math|Integer|IncrementInt (Variables|Default|GetContador)))
    (Variables|Default|SetRight 0 :!label _label)
    (Variables|Default|SetLeft 0)
    (Variables|Default|SetContador 0)
    (elif (>= (+ (* (Variables|Default|GetLeft) -1) (Variables|Default|GetRight)) 1)
      (while (< (Variables|Default|GetContador) 4)
        (Utilities|Array|RemoveIndex _hallways4thlooparray (- _returnvalue 1))
        (Math|Integer|IncrementInt (Variables|Default|GetContador)))
      (Variables|Default|SetContador 0)
      (while (< (Variables|Default|GetContador) 4)
        (Utilities|Array|Insert _hallways4thlooparray (Utilities|Array|Get(acopy) (Variables|4thLoop|GetHallway4thLoopTurns) 1) (- _returnvalue 0))
        (Math|Integer|IncrementInt (Variables|Default|GetContador)))
      (goto _label))))