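; Rooms_Proves02 is a room Blueprint that holds logic for spawning a single NPC, but that logic is disconnected and never runs.
; The unused chain checks a spawned flag on the GI_Nightmare game instance, then spawns an NPC once at an offset from the room's location.
; It sets the shared flag when the spawn is valid.
; BeginPlay and the construction script are empty.
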(event EventBeginPlay)

(fn ConstructionScript)