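; Trigger actor that shows its Mensaje text as a tutorial message by writing it to the Player's Tutorial variable while overlapped.
; When PrimerMensaje is set, overlap retries through short Delay loops until the Player exists and is Jugando, then waits briefly before writing.
; Otherwise it writes immediately if Dentro is true.
; End overlap sets Dentro false, never re-set here, and clears the text.
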(event OnComponentBeginOverlap(CollisionComponent)
  (params (OverlappedComponent :type Primitive%20Component%20Object%20Reference) (OtherActor :type Actor%20Object%20Reference) (OtherComp :type Primitive%20Component%20Object%20Reference) (OtherBodyIndex :type Integer) (bFromSweep :type Boolean) (SweepResult :type Hit%20Result%20Structure%20%28by%20ref%29))
  (bind _returnvalue (Game|GetPlayerCharacter 0))
  (if (Actor|ActorHasTag OtherActor "Player")
    (if (Variables|Default|GetPrimer_Mensaje)
      (bind _asplayer (Utilities|Casting|CastToPlayer _returnvalue :!label _label)
        (:then
          (if (Variables|/Game/MyBlueprints/Blueprints/Player/Player.Player_C|GetJugando? _asplayer) :!label _label_2
            (Utilities|FlowControl|Delay 2.0)
            (Variables|/Game/MyBlueprints/Blueprints/Player/Player.Player_C|SetTutorial _asplayer (Variables|Default|GetMensaje))
            (else
              (Utilities|FlowControl|Delay 0.2)
              (goto _label_2))))
        (:CastFailed
          (Utilities|FlowControl|Delay 0.2)
          (goto _label)))
      (elif (Variables|Default|GetDentro)
        (bind _asplayer_2 (Utilities|Casting|CastToPlayer _returnvalue))
        (Variables|/Game/MyBlueprints/Blueprints/Player/Player.Player_C|SetTutorial _asplayer_2 (Variables|Default|GetMensaje))))))

(event OnComponentEndOverlap(CollisionComponent)
  (params (OverlappedComponent :type Primitive%20Component%20Object%20Reference) (OtherActor :type Actor%20Object%20Reference) (OtherComp :type Primitive%20Component%20Object%20Reference) (OtherBodyIndex :type Integer))
  (if (Actor|ActorHasTag OtherActor "Player")
    (Variables|Default|SetDentro false)
    (bind _asplayer (Utilities|Casting|CastToPlayer (Game|GetPlayerCharacter 0)))
    (Variables|/Game/MyBlueprints/Blueprints/Player/Player.Player_C|SetTutorial _asplayer "")))

(fn ConstructionScript)