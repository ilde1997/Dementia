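; TurnsController biases the hallway pool in the GM_Proves game mode according to the imbalance between left and right turns.
; It caches the game mode on BeginPlay and compares its Left and Right counts every Tick.
; When either leads by more than two, it inserts the first (Left ahead) or second (Right ahead) HallwayTurns entry twice into HallwaysArray, repeating each frame, with debug prints.
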(event EventBeginPlay
  (bind _asgm_proves (Utilities|Casting|CastToGM_Proves (Game|GetGameMode))))

(event Collision|EventActorBeginOverlap
  (params (OtherActor :type Actor%20Object%20Reference)))

(event EventTick
  (params (DeltaSeconds :type Float%20%28single-precision%29))
  (if (> (+ (Variables|Default|GetLeft) (* (Variables|Default|GetRight) -1)) 2)
    (Development|PrintString "Hello")
    (Utilities|Array|Insert (Variables|/Game/MyBlueprints/Blueprints/GM_Proves.GM_Proves_C|GetHallwaysArray (stale EventBeginPlay _asgm_proves)) (Utilities|Array|Get(acopy) (Variables|/Game/MyBlueprints/Blueprints/GM_Proves.GM_Proves_C|GetHallwayTurns (stale EventBeginPlay _asgm_proves))) 1)
    (Utilities|Array|Insert (Variables|/Game/MyBlueprints/Blueprints/GM_Proves.GM_Proves_C|GetHallwaysArray (stale EventBeginPlay _asgm_proves)) (Utilities|Array|Get(acopy) (Variables|/Game/MyBlueprints/Blueprints/GM_Proves.GM_Proves_C|GetHallwayTurns (stale EventBeginPlay _asgm_proves))) 2)
    (else
      (Development|PrintString "Bye")
      (if (> (+ (* (Variables|Default|GetLeft) -1) (Variables|Default|GetRight)) 2)
        (Utilities|Array|Insert (Variables|/Game/MyBlueprints/Blueprints/GM_Proves.GM_Proves_C|GetHallwaysArray (stale EventBeginPlay _asgm_proves)) (Utilities|Array|Get(acopy) (Variables|/Game/MyBlueprints/Blueprints/GM_Proves.GM_Proves_C|GetHallwayTurns (stale EventBeginPlay _asgm_proves)) 1) 1)
        (Utilities|Array|Insert (Variables|/Game/MyBlueprints/Blueprints/GM_Proves.GM_Proves_C|GetHallwaysArray (stale EventBeginPlay _asgm_proves)) (Utilities|Array|Get(acopy) (Variables|/Game/MyBlueprints/Blueprints/GM_Proves.GM_Proves_C|GetHallwayTurns (stale EventBeginPlay _asgm_proves)) 1) 2)))))

(fn ConstructionScript)