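; CenterCross is an interactable puzzle actor: a cross that flips between upright and inverted.
; BeginPlay randomizes the CenterCrossPuzzleIsUp flag on GI_Nightmare and snaps the pitch to 180 when it is false.
; CInteract plays one of two rotation timelines based on that flag, then inverts it on finish.
; A DoOnce blocks further interaction until the rotation completes.
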(event EventBeginPlay
  (bind _asgi_nightmare (Utilities|Casting|CastToGI_Nightmare (Game|GetGameInstance)))
  (bind _output_get (Variables|/Game/MyBlueprints/Blueprints/GameModes/GI_Nightmare.GI_Nightmare_C|SetCenterCrossPuzzleIsUp _asgi_nightmare (Math|Random|RandomBool)))
  (if (not _output_get)
    (Transformation|SetRelativeRotation (Variables|Default|GetCenterCross) (Math|Rotator|MakeRotator 0.0 1.8e+02 0.0) false false)))

(event EventCInteract
  (bind _centercross (Variables|Default|GetCenterCross))
  (Utilities|FlowControl|DoOnce false :!label _label
    (:Completed
      (bind _asgi_nightmare (Utilities|Casting|CastToGI_Nightmare (Game|GetGameInstance)))
      (if (Variables|/Game/MyBlueprints/Blueprints/GameModes/GI_Nightmare.GI_Nightmare_C|GetCenterCrossPuzzleIsUp _asgi_nightmare)
        (bind _rotation (Timeline|RotationPitch180 PlayFromStart)
          (:Update
            (Transformation|SetRelativeRotation _centercross (Math|Rotator|MakeRotator 0.0 _rotation 0.0) false false))
          (:Finished
            (Variables|/Game/MyBlueprints/Blueprints/GameModes/GI_Nightmare.GI_Nightmare_C|SetCenterCrossPuzzleIsUp _asgi_nightmare false)
            (goto _label Reset)))
        (else
          (bind _rotation_2 (Timeline|RotationPitch0 PlayFromStart)
            (:Update
              (Transformation|SetRelativeRotation _centercross (Math|Rotator|MakeRotator 0.0 _rotation_2 0.0) false false))
            (:Finished
              (Variables|/Game/MyBlueprints/Blueprints/GameModes/GI_Nightmare.GI_Nightmare_C|SetCenterCrossPuzzleIsUp _asgi_nightmare true)
              (goto _label Reset))))))))

(fn ConstructionScript)