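; HallwayEnd5th is the end-of-hallway actor that moves the player on to Level_6Loop.
; When a Player-tagged actor enters TeleportTrigger, it resets the hallway and room counts and AI spawn flags in GI_Nightmare, shows a loading screen, then opens the level after a short delay.
; A separate FallTrigger applies damage to any Player-tagged actor that overlaps it.
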(event OnComponentBeginOverlap(FallTrigger)
  (params (OverlappedComponent :type Primitive%20Component%20Object%20Reference) (OtherActor :type Actor%20Object%20Reference) (OtherComp :type Primitive%20Component%20Object%20Reference) (OtherBodyIndex :type Integer) (bFromSweep :type Boolean) (SweepResult :type Hit%20Result%20Structure%20%28by%20ref%29))
  (if (Actor|ActorHasTag OtherActor "Player")
    (Game|Damage|ApplyDamage OtherActor 1.0 0 0)))

(event OnComponentBeginOverlap(TeleportTrigger)
  (params (OverlappedComponent :type Primitive%20Component%20Object%20Reference) (OtherActor :type Actor%20Object%20Reference) (OtherComp :type Primitive%20Component%20Object%20Reference) (OtherBodyIndex :type Integer) (bFromSweep :type Boolean) (SweepResult :type Hit%20Result%20Structure%20%28by%20ref%29))
  (if (Actor|ActorHasTag OtherActor "Player")
    (bind _asgi_nightmare (Utilities|Casting|CastToGI_Nightmare (Game|GetGameInstance)))
    (Variables|/Game/MyBlueprints/Blueprints/GameModes/GI_Nightmare.GI_Nightmare_C|SetActualHallways _asgi_nightmare 0)
    (Variables|/Game/MyBlueprints/Blueprints/GameModes/GI_Nightmare.GI_Nightmare_C|SetActualRooms _asgi_nightmare 0)
    (Variables|/Game/MyBlueprints/Blueprints/GameModes/GI_Nightmare.GI_Nightmare_C|SetAiHasAlreadySpawned _asgi_nightmare false)
    (Variables|/Game/MyBlueprints/Blueprints/GameModes/GI_Nightmare.GI_Nightmare_C|SetAiHasBeenDestroyed _asgi_nightmare false)
    (bind _returnvalue (UserInterface|CreateWidget "/Game/MyBlueprints/UI/LoadingScreen.LoadingScreen_C"))
    (UserInterface|Viewport|AddtoViewport _returnvalue 0)
    (Utilities|FlowControl|Delay 0.25)
    (Game|OpenLevel(byName) "Level_6Loop")))

(event EventBeginPlay)

(event Collision|EventActorBeginOverlap
  (params (OtherActor :type Actor%20Object%20Reference)))

(event EventTick
  (params (DeltaSeconds :type Float%20%28single-precision%29)))

(fn ConstructionScript)