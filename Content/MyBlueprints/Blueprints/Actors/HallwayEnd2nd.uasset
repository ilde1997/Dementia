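; HallwayEnd2nd is a hallway-end actor that sends the player on to the Level_3Loop level.
; When an actor tagged Player overlaps its TeleportTrigger, it checks whether the DefinitivePlayer character holds the key (TengoLlave).
; With the key, it resets the hallway and room counters and the AI spawn and destroy flags in the GI_Nightmare game instance, then opens the level.
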(event OnComponentBeginOverlap(TeleportTrigger)
  (params (OverlappedComponent :type Primitive%20Component%20Object%20Reference) (OtherActor :type Actor%20Object%20Reference) (OtherComp :type Primitive%20Component%20Object%20Reference) (OtherBodyIndex :type Integer) (bFromSweep :type Boolean) (SweepResult :type Hit%20Result%20Structure%20%28by%20ref%29))
  (if (Actor|ActorHasTag OtherActor "Player")
    (bind _asdefinitive_player (Utilities|Casting|CastToDefinitivePlayer (Game|GetPlayerCharacter 0)))
    (if (Variables|/Game/MyBlueprints/DefinitivePlayer.DefinitivePlayer_C|GetTengo_Llave _asdefinitive_player)
      (bind _asgi_nightmare (Utilities|Casting|CastToGI_Nightmare (Game|GetGameInstance)))
      (Variables|/Game/MyBlueprints/Blueprints/GameModes/GI_Nightmare.GI_Nightmare_C|SetActualHallways _asgi_nightmare 0)
      (Variables|/Game/MyBlueprints/Blueprints/GameModes/GI_Nightmare.GI_Nightmare_C|SetActualRooms _asgi_nightmare 0)
      (Variables|/Game/MyBlueprints/Blueprints/GameModes/GI_Nightmare.GI_Nightmare_C|SetAiHasAlreadySpawned _asgi_nightmare false)
      (Variables|/Game/MyBlueprints/Blueprints/GameModes/GI_Nightmare.GI_Nightmare_C|SetAiHasBeenDestroyed _asgi_nightmare false)
      (Game|OpenLevel(byName) "Level_3Loop"))))

(event EventBeginPlay)

(event Collision|EventActorBeginOverlap
  (params (OtherActor :type Actor%20Object%20Reference)))

(event EventTick
  (params (DeltaSeconds :type Float%20%28single-precision%29)))

(fn ConstructionScript)