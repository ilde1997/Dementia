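; Asylum door actor that spawns a random next room from the game mode's room array on BeginPlay, up to the game instance's room limit.
; A failed, collision-blocked spawn locks the door, so interacting shows "Locked"; otherwise interaction toggles a timeline rotation.
; A looping timeline keeps the door as the nearby player's interact target only while their Detector matches it.
; NPC overlaps snap it open, then shut after a delay.
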(event OnComponentBeginOverlap(EnemyDetection)
  (params (OverlappedComponent :type Primitive%20Component%20Object%20Reference) (OtherActor :type Actor%20Object%20Reference) (OtherComp :type Primitive%20Component%20Object%20Reference) (OtherBodyIndex :type Integer) (bFromSweep :type Boolean) (SweepResult :type Hit%20Result%20Structure%20%28by%20ref%29))
  (Utilities|Casting|CastToNPC OtherActor)
  (Transformation|SetRelativeRotation (Variables|Default|GetPuerta) "0,90.000000, 0" true false))

(event OnComponentEndOverlap(EnemyDetection)
  (params (OverlappedComponent :type Primitive%20Component%20Object%20Reference) (OtherActor :type Actor%20Object%20Reference) (OtherComp :type Primitive%20Component%20Object%20Reference) (OtherBodyIndex :type Integer))
  (Utilities|Casting|CastToNPC OtherActor)
  (Utilities|FlowControl|Delay 2.0)
  (Transformation|SetRelativeRotation (Variables|Default|GetPuerta) "0, 0, 0" true false))

(event OnComponentBeginOverlap(OpenCollider)
  (params (OverlappedComponent :type Primitive%20Component%20Object%20Reference) (OtherActor :type Actor%20Object%20Reference) (OtherComp :type Primitive%20Component%20Object%20Reference) (OtherBodyIndex :type Integer) (bFromSweep :type Boolean) (SweepResult :type Hit%20Result%20Structure%20%28by%20ref%29))
  (bind _returnvalue (Game|GetPlayerCharacter 0))
  (bind _self self)
  (if (Actor|ActorHasTag OtherActor "Player")
    (Variables|Default|SetCerca true)
    (bind _asplayer (Utilities|Casting|CastToPlayer (Game|GetPlayerCharacter 0)))
    (Variables|/Game/MyBlueprints/Player/Player.Player_C|SetObjeto _asplayer _self)
    (Variables|/Game/MyBlueprints/Player/Player.Player_C|SetInteractPbject _asplayer _self)
    (Variables|/Game/MyBlueprints/Player/Player.Player_C|SetPlayer_Inside _asplayer true)
    (Timeline|Timeline_1 PlayFromStart
      (:Update
        (if (Variables|/Game/MyBlueprints/Player/Player.Player_C|GetPlayer_Inside _asplayer)
          (bind _asplayer_2 (Utilities|Casting|CastToPlayer (Game|GetPlayerCharacter 0)))
          (if (== (Variables|/Game/MyBlueprints/Player/Player.Player_C|GetDetector _asplayer_2) (Variables|/Game/MyBlueprints/Player/Player.Player_C|GetObjeto _asplayer_2))
            (bind _asplayer_3 (Utilities|Casting|CastToPlayer _returnvalue))
            (Variables|/Game/MyBlueprints/Player/Player.Player_C|SetInteractPbject _asplayer_3 self)
            (else
              (bind _asplayer_4 (Utilities|Casting|CastToPlayer _returnvalue))
              (Variables|/Game/MyBlueprints/Player/Player.Player_C|SetInteractPbject _asplayer_4 0)))))
      (:Finished
        (if (Variables|Default|GetCerca)
          (Timeline|Timeline_1 PlayFromStart))))))

(event OnComponentEndOverlap(OpenCollider)
  (params (OverlappedComponent :type Primitive%20Component%20Object%20Reference) (OtherActor :type Actor%20Object%20Reference) (OtherComp :type Primitive%20Component%20Object%20Reference) (OtherBodyIndex :type Integer))
  (Variables|Default|SetCerca false)
  (if (Actor|ActorHasTag OtherActor "Player")
    (bind _asplayer (Utilities|Casting|CastToPlayer (Game|GetPlayerCharacter 0)))
    (Variables|/Game/MyBlueprints/Player/Player.Player_C|SetInteractPbject _asplayer 0)))

(event EventBeginPlay
  (CallFunction|SpawnNextRoom))

(event EventCInteract
  (if (Variables|Default|GetCerca)
    (if (Variables|Default|GetBloqueada)
      (bind _asplayer (Utilities|Casting|CastToPlayer (Game|GetPlayerCharacter 0)))
      (Variables|/Game/MyBlueprints/Player/Player.Player_C|SetTutorial _asplayer "Locked")
      (Utilities|FlowControl|Delay 1.0)
      (Variables|/Game/MyBlueprints/Player/Player.Player_C|SetTutorial _asplayer "")
      (else
        (Utilities|FlowControl|FlipFlop
          (:A
            (bind _rotacion (Timeline|Timeline_0 Play)
              (:Update
                (Transformation|SetRelativeRotation (Variables|Default|GetPuerta) (Math|Rotator|Lerp(Rotator) "0, 0, 0" "0,-90.000000, 0" _rotacion) false false))))
          (:B
            (Timeline|Timeline_0 Reverse)))))))

(fn ConstructionScript)

(fn SpawnNextRoom
  (bind _opencollider (Variables|Default|GetOpenCollider))
  (bind _returnvalue (Transformation|GetWorldLocation _opencollider))
  (bind _asgi_nightmare (Utilities|Casting|CastToGI_Nightmare (Game|GetGameInstance)))
  (bind _asgm_proves (Utilities|Casting|CastToGM_Proves (Game|GetGameMode)))
  (if (not (== (Variables|/Game/MyBlueprints/Blueprints/GI_Nightmare.GI_Nightmare_C|GetActualRooms _asgi_nightmare) (Variables|/Game/MyBlueprints/Blueprints/GI_Nightmare.GI_Nightmare_C|GetMaxRooms _asgi_nightmare)))
    (Math|Integer|IncrementInt (Variables|/Game/MyBlueprints/Blueprints/GI_Nightmare.GI_Nightmare_C|GetActualRooms _asgi_nightmare)
      (:%20%20
        (bind _returnvalue_2 (Game|SpawnActorfromClass (Utilities|Array|Get(acopy) (Variables|/Game/MyBlueprints/Blueprints/GM_Proves.GM_Proves_C|GetRoomsArray _asgm_proves) (Math|Random|RandomIntegerinRange 0 (- (Utilities|Array|Length (Variables|/Game/MyBlueprints/Blueprints/GM_Proves.GM_Proves_C|GetRoomsArray _asgm_proves)) 1))) (Math|Transform|MakeTransform (Math|Vector|MakeVector (.x _returnvalue) (.y _returnvalue) 0.0) (Math|Conversions|RotationFromXVector (+ "0, 0, 0" (Math|Rotator|GetRotationXVector (Transformation|GetActorRotation)))) "1,1,1") "AdjustIfPossibleButDontSpawnIfColliding" 0 0))
        (Utilities|IsValid _returnvalue_2
          (:Is%20Not%20Valid
            (Variables|Default|SetBloqueada true)
            (bind _asgm_proves_2 (Utilities|Casting|CastToGM_Proves (Game|GetGameMode)))
            (Utilities|Array|Add (Variables|/Game/MyBlueprints/Blueprints/GM_Proves.GM_Proves_C|GetEmptyRooms _asgm_proves_2) _returnvalue_2)))))))