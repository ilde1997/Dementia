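; Painting actor that can fall as a one-off event when an actor tagged Player enters its FrameTrigger volume.
; Each overlap has a random chance to enable physics on Cuadro2 and apply linear and angular impulses, then disable physics after a short delay.
; A DoOnce and the FrameHasFallen flag on GI_Nightmare prevent repeats, with the flag shared through the game instance.
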(event OnComponentBeginOverlap(FrameTrigger)
  (params (OverlappedComponent :type Primitive%20Component%20Object%20Reference) (OtherActor :type Actor%20Object%20Reference) (OtherComp :type Primitive%20Component%20Object%20Reference) (OtherBodyIndex :type Integer) (bFromSweep :type Boolean) (SweepResult :type Hit%20Result%20Structure%20%28by%20ref%29))
  (bind _cuadro2 (Variables|Default|GetCuadro2))
  (bind _asgi_nightmare (Utilities|Casting|CastToGI_Nightmare (Game|GetGameInstance)))
  (if (not (Variables|/Game/MyBlueprints/Blueprints/GameModes/GI_Nightmare.GI_Nightmare_C|GetFrameHasFallen _asgi_nightmare))
    (if (Actor|ActorHasTag OtherActor "Player")
      (if (>= (Math|Random|RandomIntegerinRange 0 10) 7)
        (Utilities|FlowControl|DoOnce false
          (:Completed
            (Physics|SetSimulatePhysics _cuadro2 true)
            (Physics|AddImpulse _cuadro2 "0,5000.000000, 0" "None" false)
            (Class|PrimitiveComponent|AddAngularImpulseinRadians _cuadro2 "5000.000000, 0, 0" "None" false)
            (bind _asgi_nightmare_2 (Utilities|Casting|CastToGI_Nightmare (Game|GetGameInstance)))
            (Variables|/Game/MyBlueprints/Blueprints/GameModes/GI_Nightmare.GI_Nightmare_C|SetFrameHasFallen _asgi_nightmare_2 true)
            (Utilities|FlowControl|Delay 2.0)
            (Physics|SetSimulatePhysics _cuadro2 false)))))))

(event EventBeginPlay)

(event Collision|EventActorBeginOverlap
  (params (OtherActor :type Actor%20Object%20Reference)))

(event EventTick
  (params (DeltaSeconds :type Float%20%28single-precision%29)))

(fn ConstructionScript)