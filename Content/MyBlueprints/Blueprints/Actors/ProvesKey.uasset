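; Key pickup actor that the player can collect while inside its PickUpRadius.
; Overlap registers the key on DefinitivePlayer and starts a self-restarting Timeline, used as a poll that sets or clears InteractPbject by comparing Player's Detector to Objeto.
; PickUpKey sets TengoLlave on Player and destroys the key if in range.
; Overlap casts to DefinitivePlayer, while polling and pickup cast to Player, with debug prints throughout.
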(event OnComponentBeginOverlap(PickUpRadius)
  (params (OverlappedComponent :type Primitive%20Component%20Object%20Reference) (OtherActor :type Actor%20Object%20Reference) (OtherComp :type Primitive%20Component%20Object%20Reference) (OtherBodyIndex :type Integer) (bFromSweep :type Boolean) (SweepResult :type Hit%20Result%20Structure%20%28by%20ref%29))
  (bind _returnvalue (Game|GetPlayerCharacter 0))
  (bind _self self)
  (if (Actor|ActorHasTag OtherActor "Player")
    (Variables|Default|SetClose true)
    (bind _asdefinitive_player (Utilities|Casting|CastToDefinitivePlayer OtherActor)
      (:then
        (Development|PrintString "Hello")
        (Variables|/Game/MyBlueprints/Blueprints/Player/Player.Player_C|SetObjeto _asdefinitive_player _self)
        (Variables|/Game/MyBlueprints/Blueprints/Player/Player.Player_C|SetInteractPbject _asdefinitive_player _self)
        (Variables|/Game/MyBlueprints/Blueprints/Player/Player.Player_C|SetPlayer_Inside _asdefinitive_player true)
        (Timeline|Timeline_0 PlayFromStart
          (:Update
            (if (Variables|/Game/MyBlueprints/Blueprints/Player/Player.Player_C|GetPlayer_Inside _asdefinitive_player)
              (bind _asplayer (Utilities|Casting|CastToPlayer (Game|GetPlayerCharacter 0)))
              (if (== (Variables|/Game/MyBlueprints/Blueprints/Player/Player.Player_C|GetDetector _asplayer) (Variables|/Game/MyBlueprints/Blueprints/Player/Player.Player_C|GetObjeto _asplayer))
                (bind _asplayer_2 (Utilities|Casting|CastToPlayer _returnvalue))
                (Variables|/Game/MyBlueprints/Blueprints/Player/Player.Player_C|SetInteractPbject _asplayer_2 self)
                (else
                  (bind _asplayer_3 (Utilities|Casting|CastToPlayer _returnvalue))
                  (Variables|/Game/MyBlueprints/Blueprints/Player/Player.Player_C|SetInteractPbject _asplayer_3 0)))))
          (:Finished
            (if (Variables|Default|GetClose)
              (Timeline|Timeline_0 PlayFromStart)))))
      (:CastFailed
        (Development|PrintString "F" true true "(R=1.000000,G=0.012710,B=0.000000,A=1.000000)")))))

(event OnComponentEndOverlap(PickUpRadius)
  (params (OverlappedComponent :type Primitive%20Component%20Object%20Reference) (OtherActor :type Actor%20Object%20Reference) (OtherComp :type Primitive%20Component%20Object%20Reference) (OtherBodyIndex :type Integer))
  (if (Actor|ActorHasTag OtherActor "Player")
    (Variables|Default|SetClose false)
    (bind _asdefinitive_player (Utilities|Casting|CastToDefinitivePlayer OtherActor)
      (:then
        (Development|PrintString "Bye")
        (Variables|/Game/MyBlueprints/Blueprints/Player/Player.Player_C|SetInteractPbject _asdefinitive_player 0))
      (:CastFailed
        (Development|PrintString "F" true true "(R=1.000000,G=0.012710,B=0.000000,A=1.000000)")))))

(event Custom|PickUpKey
  (if (Variables|Default|GetClose)
    (bind _asplayer (Utilities|Casting|CastToPlayer (Game|GetPlayerCharacter 0)))
    (Variables|/Game/MyBlueprints/Blueprints/Player/Player.Player_C|SetTengo_Llave _asplayer true)
    (Actor|DestroyActor)))

(fn ConstructionScript)