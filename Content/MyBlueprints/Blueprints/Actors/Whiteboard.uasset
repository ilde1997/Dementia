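; Interactable whiteboard actor that reports how many of the three evidence pieces the player has collected.
; On interact it switches on the evidence count in the GI_Nightmare game instance and briefly shows a progress message through the player's Tutorial text.
; With all three collected it also reveals the Newspaper, PhotoAsylum and PhotoLeader components.
; BeginPlay resets the game instance's evidence count to zero.
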(event EventCInteract
  (bind _asdefinitive_player (Utilities|Casting|CastToDefinitivePlayer (Game|GetPlayerCharacter 0)))
  (bind _asgi_nightmare (Utilities|Casting|CastToGI_Nightmare (Game|GetGameInstance)))
  (switch int (Variables|/Game/MyBlueprints/Blueprints/GameModes/GI_Nightmare.GI_Nightmare_C|GetEvidenceCollected _asgi_nightmare)
    (:Default
      (Variables|/Game/MyBlueprints/DefinitivePlayer.DefinitivePlayer_C|SetTutorial _asdefinitive_player "Some pices of evidence are missing")
      (Utilities|FlowControl|Delay 2.0)
      (Variables|/Game/MyBlueprints/DefinitivePlayer.DefinitivePlayer_C|SetTutorial _asdefinitive_player ""))
    (:0
      (Variables|/Game/MyBlueprints/DefinitivePlayer.DefinitivePlayer_C|SetTutorial _asdefinitive_player "Three pices of evidence are missing")
      (Utilities|FlowControl|Delay 2.0)
      (Variables|/Game/MyBlueprints/DefinitivePlayer.DefinitivePlayer_C|SetTutorial _asdefinitive_player ""))
    (:1
      (Variables|/Game/MyBlueprints/DefinitivePlayer.DefinitivePlayer_C|SetTutorial _asdefinitive_player "1/3")
      (Utilities|FlowControl|Delay 1.0)
      (Variables|/Game/MyBlueprints/DefinitivePlayer.DefinitivePlayer_C|SetTutorial _asdefinitive_player ""))
    (:2
      (Variables|/Game/MyBlueprints/DefinitivePlayer.DefinitivePlayer_C|SetTutorial _asdefinitive_player "2/3")
      (Utilities|FlowControl|Delay 1.0)
      (Variables|/Game/MyBlueprints/DefinitivePlayer.DefinitivePlayer_C|SetTutorial _asdefinitive_player ""))
    (:3
      (Variables|/Game/MyBlueprints/DefinitivePlayer.DefinitivePlayer_C|SetTutorial _asdefinitive_player "3/3")
      (Rendering|SetVisibility (Variables|Default|GetNewspaper) true false)
      (Rendering|SetVisibility (Variables|Default|GetPhoto_Asylum) true false)
      (Rendering|SetVisibility (Variables|Default|GetPhoto_Leader) true false)
      (Utilities|FlowControl|Delay 1.0)
      (Variables|/Game/MyBlueprints/DefinitivePlayer.DefinitivePlayer_C|SetTutorial _asdefinitive_player ""))))

(event EventBeginPlay
  (bind _asgi_nightmare (Utilities|Casting|CastToGI_Nightmare (Game|GetGameInstance)))
  (Variables|/Game/MyBlueprints/Blueprints/GameModes/GI_Nightmare.GI_Nightmare_C|SetEvidenceCollected _asgi_nightmare 0))

(fn ConstructionScript)