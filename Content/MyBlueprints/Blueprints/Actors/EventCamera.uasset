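; EventCamera is a one-shot trigger actor that turns the player's view toward an Objective actor when something overlaps it.
; The first overlap plays the PlayerRotation timeline behind a DoOnce.
; Each update sets the first player controller's control rotation to a lerp from the overlapping actor's rotation to a look-at rotation at the Objective, and prints a debug string.
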(event Collision|EventActorBeginOverlap
  (params (OtherActor :type Actor%20Object%20Reference))
  (Utilities|FlowControl|DoOnce false
    (:Completed
      (bind _playerrotator (Timeline|PlayerRotation Play)
        (:Update
          (Pawn|SetControlRotation (Game|GetPlayerController 0) (Math|Rotator|Lerp(Rotator) (Transformation|GetActorRotation OtherActor) (Math|Rotator|FindLookatRotation (Transformation|GetActorLocation OtherActor) (Transformation|GetActorLocation (Variables|Default|GetObjective))) _playerrotator))
          (Development|PrintString "CAGON LA PUTA IA"))))))

(fn ConstructionScript)