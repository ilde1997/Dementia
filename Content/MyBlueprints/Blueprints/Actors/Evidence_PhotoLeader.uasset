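; Evidence_PhotoLeader is a collectible evidence actor, a photo of "A hooded figure", that the player picks up by interacting.
; CInteract runs once through DoOnce, increments EvidenceCollected on the GI_Nightmare game instance and hides the PhotoLeader component.
; It then shows the caption briefly through DefinitivePlayer's Tutorial text, clears it after a delay and destroys itself.
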(event EventBeginPlay)

(event Collision|EventActorBeginOverlap
  (params (OtherActor :type Actor%20Object%20Reference)))

(event EventTick
  (params (DeltaSeconds :type Float%20%28single-precision%29)))

(event EventCInteract
  (Utilities|FlowControl|DoOnce false
    (:Completed
      (bind _asgi_nightmare (Utilities|Casting|CastToGI_Nightmare (Game|GetGameInstance)))
      (Math|Integer|IncrementInt (Variables|/Game/MyBlueprints/Blueprints/GameModes/GI_Nightmare.GI_Nightmare_C|GetEvidenceCollected _asgi_nightmare)
        (:%20%20
          (Development|SetHiddeninGame (Variables|Default|GetPhoto_Leader) true false)
          (bind _asdefinitive_player (Utilities|Casting|CastToDefinitivePlayer (Game|GetPlayerCharacter 0)))
          (Variables|/Game/MyBlueprints/DefinitivePlayer.DefinitivePlayer_C|SetTutorial _asdefinitive_player "A hooded figure")
          (Utilities|FlowControl|Delay 1.0)
          (Variables|/Game/MyBlueprints/DefinitivePlayer.DefinitivePlayer_C|SetTutorial _asdefinitive_player "")
          (Actor|DestroyActor))))))

(fn ConstructionScript)