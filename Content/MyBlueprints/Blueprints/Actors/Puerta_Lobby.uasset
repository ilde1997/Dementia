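; Lobby door actor that the player swings open and shut by interacting, unless it is locked or requires a mobile the player lacks.
; CInteract flip-flops a rotation timeline with an opening sound, or briefly shows "Locked" through the player's Tutorial text.
; The Detection overlap runs a looping timeline as a tick, keeping the door as interact target while the player's Detector matches it.
; CloseBehindTrigger locks the door, reversing another timeline if open.
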(event OnComponentBeginOverlap(CloseBehindTrigger)
  (params (OverlappedComponent :type Primitive%20Component%20Object%20Reference) (OtherActor :type Actor%20Object%20Reference) (OtherComp :type Primitive%20Component%20Object%20Reference) (OtherBodyIndex :type Integer) (bFromSweep :type Boolean) (SweepResult :type Hit%20Result%20Structure%20%28by%20ref%29))
  (if (Actor|ActorHasTag OtherActor "Player")
    (if (Variables|Default|GetClosed)
      (Variables|Default|SetBloqueada true)
      (else
        (bind _rotacion (Timeline|Timeline_2 Reverse)
          (:Update
            (Transformation|SetRelativeRotation (Variables|Default|GetPuerta) (Math|Rotator|Lerp(Rotator) "0, 0, 0" "0,-90.000000, 0" _rotacion) false false)
            (Variables|Default|SetBloqueada true)))))))

(event OnComponentBeginOverlap(Detection)
  (params (OverlappedComponent :type Primitive%20Component%20Object%20Reference) (OtherActor :type Actor%20Object%20Reference) (OtherComp :type Primitive%20Component%20Object%20Reference) (OtherBodyIndex :type Integer) (bFromSweep :type Boolean) (SweepResult :type Hit%20Result%20Structure%20%28by%20ref%29))
  (bind _returnvalue (Game|GetPlayerCharacter 0))
  (bind _self self)
  (if (Actor|ActorHasTag OtherActor "Player")
    (Variables|Default|SetCerca true)
    (bind _asdefinitive_player (Utilities|Casting|CastToDefinitivePlayer (Game|GetPlayerCharacter 0)))
    (Variables|/Game/MyBlueprints/DefinitivePlayer.DefinitivePlayer_C|SetObjeto _asdefinitive_player _self)
    (Variables|/Game/MyBlueprints/DefinitivePlayer.DefinitivePlayer_C|SetInteractPbject _asdefinitive_player _self)
    (Variables|/Game/MyBlueprints/DefinitivePlayer.DefinitivePlayer_C|SetPlayer_Inside _asdefinitive_player true)
    (Timeline|Timeline_1 PlayFromStart
      (:Update
        (if (Variables|/Game/MyBlueprints/DefinitivePlayer.DefinitivePlayer_C|GetPlayer_Inside _asdefinitive_player)
          (bind _asdefinitive_player_2 (Utilities|Casting|CastToDefinitivePlayer (Game|GetPlayerCharacter 0)))
          (if (== (Variables|/Game/MyBlueprints/DefinitivePlayer.DefinitivePlayer_C|GetDetector _asdefinitive_player_2) (Variables|/Game/MyBlueprints/DefinitivePlayer.DefinitivePlayer_C|GetObjeto _asdefinitive_player_2))
            (bind _asdefinitive_player_3 (Utilities|Casting|CastToDefinitivePlayer _returnvalue))
            (Variables|/Game/MyBlueprints/DefinitivePlayer.DefinitivePlayer_C|SetInteractPbject _asdefinitive_player_3 self)
            (else
              (bind _asdefinitive_player_4 (Utilities|Casting|CastToDefinitivePlayer _returnvalue))
              (Variables|/Game/MyBlueprints/DefinitivePlayer.DefinitivePlayer_C|SetInteractPbject _asdefinitive_player_4 0)))))
      (:Finished
        (if (Variables|Default|GetCerca)
          (Timeline|Timeline_1 PlayFromStart))))))

(event OnComponentEndOverlap(Detection)
  (params (OverlappedComponent :type Primitive%20Component%20Object%20Reference) (OtherActor :type Actor%20Object%20Reference) (OtherComp :type Primitive%20Component%20Object%20Reference) (OtherBodyIndex :type Integer))
  (Variables|Default|SetCerca false)
  (if (Actor|ActorHasTag OtherActor "Player")
    (bind _asdefinitive_player (Utilities|Casting|CastToDefinitivePlayer (Game|GetPlayerCharacter 0)))
    (Variables|/Game/MyBlueprints/DefinitivePlayer.DefinitivePlayer_C|SetInteractPbject _asdefinitive_player 0)))

(event EventCInteract
  (if (Variables|Default|GetCerca)
    (if (Variables|Default|GetNecesita_Movil)
      (bind _asdefinitive_player (Utilities|Casting|CastToDefinitivePlayer (Game|GetPlayerCharacter 0)))
      (if (Variables|/Game/MyBlueprints/DefinitivePlayer.DefinitivePlayer_C|GetPlayerHasMobile _asdefinitive_player)
        (if (Variables|Default|GetBloqueada) :!label _label
          (bind _asdefinitive_player_2 (Utilities|Casting|CastToDefinitivePlayer (Game|GetPlayerCharacter 0) :!label _label_2))
          (Variables|/Game/MyBlueprints/DefinitivePlayer.DefinitivePlayer_C|SetTutorial _asdefinitive_player_2 "Locked")
          (Utilities|FlowControl|Delay 1.0)
          (Variables|/Game/MyBlueprints/DefinitivePlayer.DefinitivePlayer_C|SetTutorial _asdefinitive_player_2 "")
          (else
            (Utilities|FlowControl|FlipFlop
              (:A
                (Variables|Default|SetClosed false)
                (Audio|Components|Audio|Play (Variables|Default|GetPuertaMadera_AbrirLento) 0.0)
                (bind _rotacion (Timeline|Timeline_0 Play)
                  (:Update
                    (Transformation|SetRelativeRotation (Variables|Default|GetPuerta) (Math|Rotator|Lerp(Rotator) "0, 0, 0" "0,-90.000000, 0" _rotacion) false false))))
              (:B
                (Variables|Default|SetClosed true)
                (Timeline|Timeline_0 Reverse)))))
        (else
          (goto _label_2)))
      (else
        (goto _label)))))

(fn ConstructionScript)