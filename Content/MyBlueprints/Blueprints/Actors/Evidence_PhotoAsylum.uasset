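; Evidence pickup actor for an asylum photo that the player collects through the CInteract event.
; A DoOnce gate limits collection to one trigger, which increments the evidence count on GI_Nightmare and hides the photo.
; It then shows a short caption through the DefinitivePlayer's Tutorial text, clears it after a brief delay and destroys itself.
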(event EventCInteract
  (Utilities|FlowControl|DoOnce false
    (:Completed
      (bind _asgi_nightmare (Utilities|Casting|CastToGI_Nightmare (Game|GetGameInstance)))
      (Math|Integer|IncrementInt (Variables|/Game/MyBlueprints/Blueprints/GameModes/GI_Nightmare.GI_Nightmare_C|GetEvidenceCollected _asgi_nightmare)
        (:%20%20
          (Development|SetHiddeninGame (Variables|Default|GetPhoto_Asylum) true false)
          (bind _asdefinitive_player (Utilities|Casting|CastToDefinitivePlayer (Game|GetPlayerCharacter 0)))
          (Variables|/Game/MyBlueprints/DefinitivePlayer.DefinitivePlayer_C|SetTutorial _asdefinitive_player "A hallway")
          (Utilities|FlowControl|Delay 1.0)
          (Variables|/Game/MyBlueprints/DefinitivePlayer.DefinitivePlayer_C|SetTutorial _asdefinitive_player "")
          (Actor|DestroyActor))))))

(fn ConstructionScript)