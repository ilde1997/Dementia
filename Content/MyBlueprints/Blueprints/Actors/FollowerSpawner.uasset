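; Trigger actor that spawns an AI_Follower when a Player-tagged actor overlaps its SpawnTrigger.
; A DoOnce gates the spawn, which follows a short random delay and a 2D sound and lands at the SpawnPosition transform.
; Spawned and destroyed flags on GI_Nightmare prevent duplicate followers.
; An overlap after the follower's destruction clears the spawned flag and resets that spawner's gate.
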(event OnComponentBeginOverlap(SpawnTrigger)
  (params (OverlappedComponent :type Primitive%20Component%20Object%20Reference) (OtherActor :type Actor%20Object%20Reference) (OtherComp :type Primitive%20Component%20Object%20Reference) (OtherBodyIndex :type Integer) (bFromSweep :type Boolean) (SweepResult :type Hit%20Result%20Structure%20%28by%20ref%29))
  (if (Actor|ActorHasTag OtherActor "Player")
    (bind _asgi_nightmare (Utilities|Casting|CastToGI_Nightmare (Game|GetGameInstance)))
    (if (Variables|/Game/MyBlueprints/Blueprints/GI_Nightmare.GI_Nightmare_C|GetAiHasAlreadySpawned _asgi_nightmare)
      (if (Variables|/Game/MyBlueprints/Blueprints/GI_Nightmare.GI_Nightmare_C|GetAiHasBeenDestroyed _asgi_nightmare)
        (Variables|/Game/MyBlueprints/Blueprints/GI_Nightmare.GI_Nightmare_C|SetAiHasAlreadySpawned _asgi_nightmare false)
        (goto _label Reset))
      (else
        (Utilities|FlowControl|DoOnce false :!label _label
          (:Completed
            (Utilities|FlowControl|Delay (Math|Random|RandomFloatinRange 0.1 0.5))
            (Audio|PlaySound2D "/Engine/EditorSounds/Notifications/CompileSuccess.CompileSuccess" 1.0 1.0 0.0 0 0)
            (Game|SpawnActorfromClass "/Game/AI/AI_Follower.AI_Follower_C" (Transformation|GetWorldTransform (Variables|Default|GetSpawnPosition)) "Undefined" 0 0)
            (Variables|/Game/MyBlueprints/Blueprints/GI_Nightmare.GI_Nightmare_C|SetAiHasAlreadySpawned _asgi_nightmare true)
            (Variables|/Game/MyBlueprints/Blueprints/GI_Nightmare.GI_Nightmare_C|SetAiHasBeenDestroyed _asgi_nightmare false)))))))

(event EventBeginPlay)

(event Collision|EventActorBeginOverlap
  (params (OtherActor :type Actor%20Object%20Reference)))

(event EventTick
  (params (DeltaSeconds :type Float%20%28single-precision%29)))

(fn ConstructionScript)