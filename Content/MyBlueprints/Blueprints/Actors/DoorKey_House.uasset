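; House door that the player opens and closes through interaction, provided they are nearby and hold the key.
; CInteract alternates timeline-driven swings via FlipFlop, signing the opening angle by the player-to-door Z direction, or shows a brief locked or needs-key message.
; A detection overlap handles proximity and interact-target registration.
; A close-behind trigger locks the door, shutting it if open, then destroying AI_Follower actors and flagging GI_Nightmare.
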(event OnComponentBeginOverlap(CloseBehindTrigger)
  (params (OverlappedComponent :type Primitive%20Component%20Object%20Reference) (OtherActor :type Actor%20Object%20Reference) (OtherComp :type Primitive%20Component%20Object%20Reference) (OtherBodyIndex :type Integer) (bFromSweep :type Boolean) (SweepResult :type Hit%20Result%20Structure%20%28by%20ref%29))
  (if (Actor|ActorHasTag OtherActor "Player")
    (if (Variables|Default|GetClosed)
      (Variables|Default|SetBloqueada true)
      (else
        (bind _rotacion (Timeline|Timeline_4 PlayFromStart)
          (:Update
            (Transformation|SetRelativeRotation (Variables|Default|GetPuerta) (Math|Rotator|Lerp(Rotator) "0, 0, 0" "0,-90.000000, 0" _rotacion) false false)
            (Variables|Default|SetClosed true)
            (Variables|Default|SetBloqueada true))
          (:Finished
            (Audio|PlaySound2D "/Game/MyBlueprints/Sound/Cues/SC_CloseDoor.SC_CloseDoor" 1.0 1.0 0.0 0 0)
            (bind _outactors (Actor|GetAllActorsOfClass "/Game/AI/AI_Follower.AI_Follower_C"))
            (for _array_element _outactors
              (Default|AiSelfDestroy _array_element))
            (bind _asgi_nightmare (Utilities|Casting|CastToGI_Nightmare (Game|GetGameInstance)))
            (Variables|/Game/MyBlueprints/Blueprints/GameModes/GI_Nightmare.GI_Nightmare_C|SetAiHasBeenDestroyed _asgi_nightmare true)))))))

(event OnComponentBeginOverlap(Detection)
  (params (OverlappedComponent :type Primitive%20Component%20Object%20Reference) (OtherActor :type Actor%20Object%20Reference) (OtherComp :type Primitive%20Component%20Object%20Reference) (OtherBodyIndex :type Integer) (bFromSweep :type Boolean) (SweepResult :type Hit%20Result%20Structure%20%28by%20ref%29))
  (bind _self self)
  (if (Actor|ActorHasTag OtherActor "Player")
    (Variables|Default|SetCerca true)
    (bind _asdefinitive_player (Utilities|Casting|CastToDefinitivePlayer (Game|GetPlayerCharacter 0)))
    (if (== _self (Variables|/Game/MyBlueprints/DefinitivePlayer.DefinitivePlayer_C|GetDetector _asdefinitive_player))
      (Variables|/Game/MyBlueprints/DefinitivePlayer.DefinitivePlayer_C|SetInteractPbject _asdefinitive_player _self))))

(event OnComponentEndOverlap(Detection)
  (params (OverlappedComponent :type Primitive%20Component%20Object%20Reference) (OtherActor :type Actor%20Object%20Reference) (OtherComp :type Primitive%20Component%20Object%20Reference) (OtherBodyIndex :type Integer))
  (Variables|Default|SetCerca false)
  (if (Actor|ActorHasTag OtherActor "Player")
    (bind _asdefinitive_player (Utilities|Casting|CastToDefinitivePlayer (Game|GetPlayerCharacter 0)))
    (Variables|/Game/MyBlueprints/DefinitivePlayer.DefinitivePlayer_C|SetInteractPbject _asdefinitive_player 0)))

(event EventCInteract
  (if (and (Variables|Default|GetCerca) (not (Variables|Default|GetAnimation)))
    (bind _asdefinitive_player (Utilities|Casting|CastToDefinitivePlayer (Game|GetPlayerCharacter 0)))
    (if (Variables|/Game/MyBlueprints/DefinitivePlayer.DefinitivePlayer_C|GetTengo_Llave _asdefinitive_player)
      (if (Variables|Default|GetBloqueada)
        (bind _asdefinitive_player_2 (Utilities|Casting|CastToDefinitivePlayer (Game|GetPlayerCharacter 0)))
        (Variables|/Game/MyBlueprints/DefinitivePlayer.DefinitivePlayer_C|SetTutorial _asdefinitive_player_2 "Locked")
        (Audio|PlaySound2D "/Game/MyBlueprints/Sound/Waves/S_LockedDoor_01.S_LockedDoor_01" 1.0 1.0 0.0 0 0)
        (Utilities|FlowControl|Delay 1.0)
        (Variables|/Game/MyBlueprints/DefinitivePlayer.DefinitivePlayer_C|SetTutorial _asdefinitive_player_2 "")
        (else
          (bind _asdefinitive_player_3 (Utilities|Casting|CastToDefinitivePlayer (Game|GetPlayerCharacter 0)))
          (Variables|Default|SetAnimation true)
          (Utilities|FlowControl|FlipFlop
            (:A
              (Audio|PlaySound2D "/Game/MyBlueprints/Sound/Waves/S_Open_Door_01.S_Open_Door_01" 1.0 1.0 0.0 0 0)
              (Development|PrintString (Utilities|String|ToString(Float) (Math|Float|Sign(Float) (.z (Math|Vector|GetUnitDirection(Vector) (Transformation|GetActorLocation _asdefinitive_player_3) (Transformation|GetActorLocation))))))
              (bind _rotacion (Timeline|Timeline_1 PlayFromStart)
                (:Update
                  (Transformation|SetRelativeRotation (Variables|Default|GetPuerta) (Math|Rotator|Lerp(Rotator) "0, 0, 0" "0,-90.000000, 0" (* _rotacion (Math|Float|Sign(Float) (.z (Math|Vector|GetUnitDirection(Vector) (Transformation|GetActorLocation _asdefinitive_player_3) (Transformation|GetActorLocation)))))) false false))
                (:Finished
                  (Variables|Default|SetClosed false)
                  (Variables|Default|SetAnimation false))))
            (:B
              (bind _rotacion_2 (Timeline|Timeline_2 PlayFromStart)
                (:Update
                  (Transformation|SetRelativeRotation (Variables|Default|GetPuerta) (Math|Rotator|Lerp(Rotator) "0, 0, 0" "0,-90.000000, 0" _rotacion_2) false false))
                (:Finished
                  (Audio|PlaySound2D "/Game/MyBlueprints/Sound/Cues/SC_CloseDoor.SC_CloseDoor" 1.0 1.0 0.0 0 0)
                  (Variables|Default|SetClosed true)
                  (Variables|Default|SetAnimation false)))))))
      (else
        (bind _asdefinitive_player_4 (Utilities|Casting|CastToDefinitivePlayer (Game|GetPlayerCharacter 0)))
        (Variables|/Game/MyBlueprints/DefinitivePlayer.DefinitivePlayer_C|SetTutorial _asdefinitive_player_4 "It needs a key")
        (Audio|PlaySound2D "/Game/MyBlueprints/Sound/Waves/S_LockedDoor_01.S_LockedDoor_01" 1.0 1.0 0.0 0 0)
        (Utilities|FlowControl|Delay 1.0)
        (Variables|/Game/MyBlueprints/DefinitivePlayer.DefinitivePlayer_C|SetTutorial _asdefinitive_player_4 "")))))

(fn ConstructionScript)