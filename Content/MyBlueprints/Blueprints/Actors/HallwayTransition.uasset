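; Hallway transition actor that swaps itself for the Lobby2ndLoop actor when the player walks through it.
; When an actor tagged Player overlaps TriggerSpawnDestroy, it waits briefly, spawns the lobby and destroys itself.
; The lobby is placed at DoorThingy's X/Y on world Z zero, facing along the hallway actor's forward vector, with spawn collision ignored.
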(event OnComponentBeginOverlap(TriggerSpawnDestroy)
  (params (OverlappedComponent :type Primitive%20Component%20Object%20Reference) (OtherActor :type Actor%20Object%20Reference) (OtherComp :type Primitive%20Component%20Object%20Reference) (OtherBodyIndex :type Integer) (bFromSweep :type Boolean) (SweepResult :type Hit%20Result%20Structure%20%28by%20ref%29))
  (bind _doorthingy (Variables|Default|GetDoorThingy))
  (bind _returnvalue (Transformation|GetWorldLocation _doorthingy))
  (if (Actor|ActorHasTag OtherActor "Player")
    (Utilities|FlowControl|Delay 0.4)
    (Game|SpawnActorfromClass "/Game/MyBlueprints/Actores/Habitaciones_Enteras/Lobby2ndLoop.Lobby2ndLoop_C" (Math|Transform|MakeTransform (Math|Vector|MakeVector (.x _returnvalue) (.y _returnvalue) 0.0) (Math|Conversions|RotationFromXVector (+ "0, 0, 0" (Math|Rotator|GetRotationXVector (Transformation|GetActorRotation)))) "1,1,1") "AlwaysSpawn" 0 0)
    (Actor|DestroyActor)))

(event EventBeginPlay)

(event Collision|EventActorBeginOverlap
  (params (OtherActor :type Actor%20Object%20Reference)))

(event EventTick
  (params (DeltaSeconds :type Float%20%28single-precision%29)))

(fn ConstructionScript)